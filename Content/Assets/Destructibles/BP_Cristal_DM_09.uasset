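; Destructible crystal actor that breaks when a magic projectile hits it and spawns a B_Cristal actor at its location.
; Overlap of the Er component with BP_ProyectilMagico applies impulse damage to the Cristal destructible component and spawns B_Cristal.
; Hits on Cristal also spawn B_Cristal, gated by a Destroyed flag that starts true and toggles each hit, so only alternate hits spawn.
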(event `self.ReceiveHit`
  (params (MyComp :type "PrimitiveComponent Object Reference") (Other :type "Actor Object Reference") (OtherComp :type "PrimitiveComponent Object Reference") (bSelfMoved :type Boolean) (HitLocation :type "Vector Structure") (HitNormal :type "Vector Structure") (NormalImpulse :type "Vector Structure") (Hit :type "HitResult Structure (by ref)")))

(event `self.ReceiveBeginPlay`
  (set `self.Destroyed` true))

(event `self.Cristal.OnComponentHit`
  (params (HitComponent :type "PrimitiveComponent Object Reference") (OtherActor :type "Actor Object Reference") (OtherComp :type "PrimitiveComponent Object Reference") (NormalImpulse :type "Vector Structure") (Hit :type "HitResult Structure (by ref)"))
  (if (`self.Destroyed`)
    (`|SpawnActorFromClass` "/Game/Materiales/B_Cristal.B_Cristal_C" (`KismetMathLibrary.Conv_VectorToTransform` (`self.K2_GetActorLocation` self)) "AdjustIfPossibleButAlwaysSpawn" "OverrideRootScale" null null)
    (set `self.Destroyed` false)
    (else
      (set `self.Destroyed` true))))

(event `self.er.OnComponentBeginOverlap`
  (params (OverlappedComponent :type "PrimitiveComponent Object Reference") (OtherActor :type "Actor Object Reference") (OtherComp :type "PrimitiveComponent Object Reference") (OtherBodyIndex :type Integer) (bFromSweep :type Boolean) (SweepResult :type "HitResult Structure (by ref)"))
  (bind (_bblockinghit _binitialoverlap _time _distance _location _impactpoint) (`GameplayStatics.BreakHitResult` SweepResult))
  (cast `/Game/Materiales2/BP_ProyectilMagico` OtherActor)
  (`DestructibleComponent.ApplyDamage` (`self.Cristal`) 0.0 _location _impactpoint 200.0)
  (`|SpawnActorFromClass` "/Game/Materiales/B_Cristal.B_Cristal_C" (`KismetMathLibrary.Conv_VectorToTransform` (`self.K2_GetActorLocation` self)) "AdjustIfPossibleButAlwaysSpawn" "OverrideRootScale" null null))

(fn `UserConstructionScript`)