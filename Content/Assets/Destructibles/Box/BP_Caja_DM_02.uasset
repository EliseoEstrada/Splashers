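; Destructible box that reacts to water bullets and to contact with the player character.
; A BP_WaterBullet overlapping the Colicion component applies damage to the Caja destructible with a fixed hit location and strong fixed impulse.
; A ThirdPersonCharacter hitting Caja destroys the whole actor after a one-second delay.
; BeginPlay sets a Destroyed flag that nothing in this graph reads.
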(event `self.ReceiveHit`
  (params (MyComp :type "PrimitiveComponent Object Reference") (Other :type "Actor Object Reference") (OtherComp :type "PrimitiveComponent Object Reference") (bSelfMoved :type Boolean) (HitLocation :type "Vector Structure") (HitNormal :type "Vector Structure") (NormalImpulse :type "Vector Structure") (Hit :type "HitResult Structure (by ref)")))

(event `self.ReceiveBeginPlay`
  (set `self.Destroyed` true))

(event `self.Caja.OnComponentHit`
  (params (HitComponent :type "PrimitiveComponent Object Reference") (OtherActor :type "Actor Object Reference") (OtherComp :type "PrimitiveComponent Object Reference") (NormalImpulse :type "Vector Structure") (Hit :type "HitResult Structure (by ref)"))
  (cast `/Game/ThirdPersonBP/Blueprints/ThirdPersonCharacter` OtherActor)
  (`KismetSystemLibrary.Delay` 1.0)
  (`self.K2_DestroyActor`))

(event `self.colicion.OnComponentBeginOverlap`
  (params (OverlappedComponent :type "PrimitiveComponent Object Reference") (OtherActor :type "Actor Object Reference") (OtherComp :type "PrimitiveComponent Object Reference") (OtherBodyIndex :type Integer) (bFromSweep :type Boolean) (SweepResult :type "HitResult Structure (by ref)"))
  (cast `/Game/Blueprints/Gameplay/BP_WaterBullet` OtherActor)
  (`DestructibleComponent.ApplyDamage` (`self.Caja`) 0.0 (-100.0 -100.0 0.0) (100.0 100.0 0.0) 2000.0))

(fn `UserConstructionScript`)