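; Water bullet projectile that damages ThirdPersonCharacters on overlap and expires after a short lifespan.
; On spawn it plays a shot sound; the BigProyectil flag swaps in the giant cue, enlarges the actor and doubles Damage.
; Overlapping a character other than the Instigator routes damage through the victim's BP_PlayerController, crediting the Instigator, then destroys the bullet.
; Other actors are ignored.
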(event `self.ReceiveBeginPlay`
  (bind _returnvalue (`self.K2_GetActorLocation`))
  (`self.SetLifeSpan` 2.0)
  (if (`self.BigProyectil`)
    (`GameplayStatics.SpawnSoundAtLocation` "/Game/Assets/Audio/Efectos/Disparo_Gigante_Cue.Disparo_Gigante_Cue" _returnvalue (struct) 1.0 1.0 0.0 null null)
    (`self.SetActorScale3D` self (3.0 3.0 3.0))
    (set `self.Damage` (* (`self.Damage`) 2.0))
    (else
      (`GameplayStatics.SpawnSoundAtLocation` "/Game/Assets/Audio/Efectos/Disparo_Cue.Disparo_Cue" _returnvalue (struct) 1.0 1.0 0.0 null null))))

(event `self.Collision.OnComponentBeginOverlap`
  (params (OverlappedComponent :type "PrimitiveComponent Object Reference") (OtherActor :type "Actor Object Reference") (OtherComp :type "PrimitiveComponent Object Reference") (OtherBodyIndex :type Integer) (bFromSweep :type Boolean) (SweepResult :type "HitResult Structure (by ref)"))
  (bind _asthird_person_character (cast `/Game/ThirdPersonBP/Blueprints/ThirdPersonCharacter` OtherActor)
    (:`then`
      (`/Engine/EditorBlueprintResources/StandardMacros.IsValid` _asthird_person_character
        (:`Is Valid`
          (if (!= OtherActor (`self.Instigator`))
            (bind _asbp_player_controller (cast `/Game/Blueprints/Main/BP_PlayerController` (`Pawn.GetController` _asthird_person_character)))
            (`/Game/Blueprints/Main/BP_PlayerController.Apply Damage` _asbp_player_controller _asthird_person_character (`self.Instigator`) (`self.Damage`))
            (`self.K2_DestroyActor` :!label _label)))
        (:`Is Not Valid`
          (goto _label))))
    (:`CastFailed`
      (if (== OtherActor self)
        _))))

(fn `UserConstructionScript`)