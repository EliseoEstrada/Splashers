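; Lobby game mode that registers joining players and handles swapping their playable character.
; After a short delay on login, it adds each BP_Lobby_PC to a Players list and sends it the transform of a player start named after the current player count.
; SwapCharacter destroys the controller's current pawn, spawns the chosen Smol character class at the supplied transform, and possesses it, defaulting to Smolkiara.
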(event `self.K2_PostLogin`
  (params (NewPlayer :type "PlayerController Object Reference"))
  (`KismetSystemLibrary.Delay` 0.05)
  (bind _asbp_lobby_pc (cast `/Game/Blueprints/Lobby/BP_Lobby_PC` NewPlayer))
  (`KismetArrayLibrary.Array_Add` (`self.Players`) _asbp_lobby_pc)
  (`/Game/Blueprints/Lobby/BP_Lobby_PC.Client Post Login` _asbp_lobby_pc (`self.GetTransform` (`self.K2_FindPlayerStart` NewPlayer (`KismetStringLibrary.Conv_IntToString` (`KismetArrayLibrary.Array_Length` (`self.Players`)))))))

(event `Swap Character`
  (params (PlayerController :type "PlayerController Object Reference") (Character :type "Object Class Reference") (Transform :type "Transform Structure"))
  ;[0.4011 0.184 1] Cambiar de personaje
  (`self.Asign Character Spawn` PlayerController Character Transform))

(fn `Asign Character Spawn`
  (params (PlayerController :type "PlayerController Object Reference") (Character :type "Object Class Reference") (Transform :type "Transform Structure"))
  (`/Engine/EditorBlueprintResources/StandardMacros.IsValid` PlayerController
    (:`Is Valid`
      (bind _asbp_lobby_pc (cast `/Game/Blueprints/Lobby/BP_Lobby_PC` PlayerController))
      (bind _returnvalue (`Controller.K2_GetPawn` _asbp_lobby_pc))
      (set `self.Spawn transform` (`self.GetTransform` _returnvalue))
      (`self.K2_DestroyActor` _returnvalue)
      (if (== Character "/Game/Blueprints/Characters/Smolame.Smolame_C")
        (bind _returnvalue_2 (`|SpawnActorFromClass` "/Game/Blueprints/Characters/Smolame.Smolame_C" Transform "Undefined" "OverrideRootScale" null null))
        (`Controller.Possess` PlayerController _returnvalue_2)
        (elif (== Character "/Game/Blueprints/Characters/Smolcalli.Smolcalli_C")
          (bind _returnvalue_3 (`|SpawnActorFromClass` "/Game/Blueprints/Characters/Smolcalli.Smolcalli_C" Transform "Undefined" "OverrideRootScale" null null))
          (`Controller.Possess` PlayerController _returnvalue_3)
          (elif (== Character "/Game/Blueprints/Characters/Smolgura.Smolgura_C")
            (bind _returnvalue_4 (`|SpawnActorFromClass` "/Game/Blueprints/Characters/Smolgura.Smolgura_C" Transform "Undefined" "OverrideRootScale" null null))
            (`Controller.Possess` PlayerController _returnvalue_4)
            (elif (== Character "/Game/Blueprints/Characters/Smolina.Smolina_C")
              (bind _returnvalue_5 (`|SpawnActorFromClass` "/Game/Blueprints/Characters/Smolina.Smolina_C" Transform "Undefined" "OverrideRootScale" null null))
              (`Controller.Possess` PlayerController _returnvalue_5)
              (else
                (bind _returnvalue_6 (`|SpawnActorFromClass` "/Game/Blueprints/Characters/Smolkiara.Smolkiara_C" Transform "Undefined" "OverrideRootScale" null null))
                (`Controller.Possess` PlayerController _returnvalue_6)))))))))

(fn `UserConstructionScript`)