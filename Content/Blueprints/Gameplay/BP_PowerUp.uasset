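; BP_PowerUp is a one-shot pickup that grants the player a big-projectile power-up.
; When a ThirdPersonCharacter overlaps its box, it sets the big-projectile flag and power-up time on that player's BP_PlayerState.
; It then plays a sound and particle effect and destroys itself after a short delay, with an Active flag blocking repeat triggers.
; A timeline for spinning the mesh exists but never runs.
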(event `self.Box.OnComponentBeginOverlap`
  (params (OverlappedComponent :type "PrimitiveComponent Object Reference") (OtherActor :type "Actor Object Reference") (OtherComp :type "PrimitiveComponent Object Reference") (OtherBodyIndex :type Integer) (bFromSweep :type Boolean) (SweepResult :type "HitResult Structure (by ref)"))
  (if (not (`self.active`))
    (cast `/Game/ThirdPersonBP/Blueprints/ThirdPersonCharacter` OtherActor)
    (bind _asbp_player_controller (cast `/Game/Blueprints/Main/BP_PlayerController` (`self.GetInstigatorController` OtherActor)))
    (set `self.active` true)
    (bind _asbp_player_state (cast `/Game/Blueprints/Main/BP_PlayerState` (`Controller.PlayerState` _asbp_player_controller)))
    (set `/Game/Blueprints/Main/BP_PlayerState.Big Proyectil` true _asbp_player_state)
    (set `/Game/Blueprints/Main/BP_PlayerState.Time Power Up` 100.0 _asbp_player_state)
    (`GameplayStatics.PlaySound2D` "/Game/Assets/Audio/Musica/power_up.power_up" 1.0 1.0 0.0 null null)
    (`GameplayStatics.SpawnEmitterAtLocation` "/Game/Particulas/PS_Health.PS_Health" (`self.K2_GetActorLocation` self))
    (`KismetSystemLibrary.Delay` 1.0)
    (`self.K2_DestroyActor`)))

(fn `UserConstructionScript`)