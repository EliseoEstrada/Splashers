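; Game mode for a timed multiplayer match with selectable Smol characters, driving players through client calls on BP_PlayerController.
; PostLogin registers each player and passes a numbered PlayerStart; after BeginPlay a countdown enables input and starts the match.
; A looping timer decrements the GameState clock, freezing input at zero.
; Character swaps and mid-match respawns destroy the current pawn, then spawn and possess the chosen class, with respawns using random PlayerStarts.
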(event `self.ReceiveBeginPlay`
  (`GameplayStatics.PlaySound2D` "/Game/Assets/Audio/Musica/Música_juego2.Música_juego2" 0.5 1.0 0.0 null null)
  (`KismetSystemLibrary.Delay` 2.0)
  (bind _asbp_game_state (cast `/Game/Blueprints/Main/BP_GameState` (`GameplayStatics.GetGameState`)))
  (set `self.BP GS` _asbp_game_state)
  (`self.Countdown`))

(event `Swap Character`
  (params (PlayerController :type "PlayerController Object Reference") (Character :type "Object Class Reference") (Location :type "Transform Structure"))
  (`self.Asign Character Spawn` PlayerController Character Location)
  (bind _asbp_player_controller (cast `/Game/Blueprints/Main/BP_PlayerController` PlayerController))
  (`/Game/Blueprints/Main/BP_PlayerController.Client Enable Input` _asbp_player_controller false))

(event `Countdown`
  ;[1 1 1] Cuenta regresiva de inicio de partida
  (for _ (`self.Players`)
    (`self.Show Countdown`))
  (`KismetSystemLibrary.Delay` 3.0)
  (set `self.Started` true)
  (`self.Unfreeze`)
  ;[1 1 1] Iniciar tiempo de partida
  (set `/Game/Blueprints/Main/BP_GameState.CurrentTime` (`self.MaxTimeServer`) (`self.BP GS`))
  (bind _returnvalue (`KismetSystemLibrary.K2_SetTimerDelegate` (delegate `Count`) 1.0 true))
  (`self.Show Timers`))

(event `self.K2_PostLogin`
  (params (NewPlayer :type "PlayerController Object Reference"))
  ;[1 0.1141 0.1041] Spawnear jugardor al inicio de partida
  (`KismetSystemLibrary.Delay` 0.05)
  (bind _asbp_player_controller (cast `/Game/Blueprints/Main/BP_PlayerController` NewPlayer))
  (`KismetArrayLibrary.Array_Add` (`self.Players`) _asbp_player_controller)
  (`/Game/Blueprints/Main/BP_PlayerController.Client Post Login` _asbp_player_controller (`self.GetTransform` (`self.K2_FindPlayerStart` NewPlayer (`KismetStringLibrary.Conv_IntToString` (`KismetArrayLibrary.Array_Length` (`self.Players`))))))
  (`/Game/Blueprints/Main/BP_PlayerController.Client Draw HUD` _asbp_player_controller))

(event `Count`
  ;[1 1 1] Iniciar tiempo de partida
  (bind _result (`/Engine/EditorBlueprintResources/StandardMacros.DecrementInt` (`/Game/Blueprints/Main/BP_GameState.CurrentTime` (`self.BP GS`)))
    (:`  `
      (if (== _result 0)
        (`KismetSystemLibrary.K2_PauseTimerHandle` (stale `Countdown` _returnvalue))
        (set `self.Started` false)
        (`self.Freeze`)))))

(event `Freeze`
  ;[1 1 1] Desactivar input a cada jugador
  (for _array_element (`self.Players`)
    (`/Game/Blueprints/Main/BP_PlayerController.Client Enable Input` _array_element false)))

(event `Respawn Requested`
  (params (PlayerController :type "PlayerController Object Reference") (Character :type "Object Class Reference"))
  ;[0.4011 0.184 1] Respawnear jugador
  (`/Engine/EditorBlueprintResources/StandardMacros.IsValid` PlayerController
    (:`Is Valid`
      (if (`self.Started`)
        (bind _position (`self.Random Player Start`))
        (`self.Asign Character Spawn` PlayerController Character _position)))))

(event `Unfreeze`
  ;[1 1 1] Activar inputs a cada jugador
  (for _array_element (`self.Players`)
    (`/Game/Blueprints/Main/BP_PlayerController.Client Enable Input` _array_element true)))

(event `Show Countdown`
  ;[0.1703 0.4623 1] Mostrar cuenta regresiva a cada jugador
  (for _array_element (`self.Players`)
    (`/Game/Blueprints/Main/BP_PlayerController.Client Show Countdown` _array_element)))

(event `Show Timers`
  ;[0.1703 0.4623 1] Mostrar tiempo de partida a cada jugador
  (for _array_element (`self.Players`)
    (`/Game/Blueprints/Main/BP_PlayerController.Client Show Time Game` _array_element)))

(fn `Asign Character Spawn`
  (params (`Player Controller` :type "PlayerController Object Reference") (Character :type "Object Class Reference") (Location :type "Transform Structure"))
  (`/Engine/EditorBlueprintResources/StandardMacros.IsValid` `Player Controller`
    (:`Is Valid`
      (bind _asbp_player_controller (cast `/Game/Blueprints/Main/BP_PlayerController` `Player Controller`))
      (bind _returnvalue (`Controller.K2_GetPawn` _asbp_player_controller))
      (`/Engine/EditorBlueprintResources/StandardMacros.IsValid` _returnvalue
        (:`Is Valid`
          (`self.K2_DestroyActor` _returnvalue))
        (:`Is Not Valid`
          _))
      (if (== Character "/Game/Blueprints/Characters/Smolame.Smolame_C")
        (bind _returnvalue_2 (`|SpawnActorFromClass` "/Game/Blueprints/Characters/Smolame.Smolame_C" Location "Undefined" "OverrideRootScale" null null))
        (`Controller.Possess` `Player Controller` _returnvalue_2)
        (elif (== Character "/Game/Blueprints/Characters/Smolcalli.Smolcalli_C")
          (bind _returnvalue_3 (`|SpawnActorFromClass` "/Game/Blueprints/Characters/Smolcalli.Smolcalli_C" Location "Undefined" "OverrideRootScale" null null))
          (`Controller.Possess` `Player Controller` _returnvalue_3)
          (elif (== Character "/Game/Blueprints/Characters/Smolgura.Smolgura_C")
            (bind _returnvalue_4 (`|SpawnActorFromClass` "/Game/Blueprints/Characters/Smolgura.Smolgura_C" Location "Undefined" "OverrideRootScale" null null))
            (`Controller.Possess` `Player Controller` _returnvalue_4)
            (elif (== Character "/Game/Blueprints/Characters/Smolina.Smolina_C")
              (bind _returnvalue_5 (`|SpawnActorFromClass` "/Game/Blueprints/Characters/Smolina.Smolina_C" Location "Undefined" "OverrideRootScale" null null))
              (`Controller.Possess` `Player Controller` _returnvalue_5)
              (else
                (bind _returnvalue_6 (`|SpawnActorFromClass` "/Game/Blueprints/Characters/Smolkiara.Smolkiara_C" Location "Undefined" "OverrideRootScale" null null))
                (`Controller.Possess` `Player Controller` _returnvalue_6)))))))))

(fn `Random Player Start`
  (returns (Position :type "Transform Structure"))
  (bind _outactors (`GameplayStatics.GetAllActorsOfClass` "/Script/Engine.PlayerStart"))
  (return (`self.GetTransform` (`|GetArrayItem` _outactors (`KismetMathLibrary.RandomIntegerInRange` 0 (- (`KismetArrayLibrary.Array_Length` _outactors) 1))))))

(fn `UserConstructionScript`)