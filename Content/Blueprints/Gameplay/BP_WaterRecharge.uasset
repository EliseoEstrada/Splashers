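; BP_WaterRecharge is a trigger-volume actor that marks players as reloading while they stand inside it, presumably to refill water.
; Box collision begin and end overlaps cast the overlapping actor to ThirdPersonCharacter, then set the Reloading flag on its BP_PlayerState true or false.
; The refill itself is not handled here, and entering also prints the character's name.
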(event `self.BoxCollision.OnComponentBeginOverlap`
  (params (OverlappedComponent :type "PrimitiveComponent Object Reference") (OtherActor :type "Actor Object Reference") (OtherComp :type "PrimitiveComponent Object Reference") (OtherBodyIndex :type Integer) (bFromSweep :type Boolean) (SweepResult :type "HitResult Structure (by ref)"))
  (bind _asthird_person_character (cast `/Game/ThirdPersonBP/Blueprints/ThirdPersonCharacter` OtherActor))
  (`/Engine/EditorBlueprintResources/StandardMacros.IsValid` _asthird_person_character
    (:`Is Valid`
      (bind _asbp_player_state (cast `/Game/Blueprints/Main/BP_PlayerState` (`Pawn.PlayerState` _asthird_person_character)))
      (`KismetSystemLibrary.PrintString` (`KismetSystemLibrary.GetDisplayName` _asthird_person_character))
      (set `/Game/Blueprints/Main/BP_PlayerState.Reloading` true _asbp_player_state))))

(event `self.BoxCollision.OnComponentEndOverlap`
  (params (OverlappedComponent :type "PrimitiveComponent Object Reference") (OtherActor :type "Actor Object Reference") (OtherComp :type "PrimitiveComponent Object Reference") (OtherBodyIndex :type Integer))
  (bind _asthird_person_character (cast `/Game/ThirdPersonBP/Blueprints/ThirdPersonCharacter` OtherActor))
  (`/Engine/EditorBlueprintResources/StandardMacros.IsValid` _asthird_person_character
    (:`Is Valid`
      (bind _asbp_player_state (cast `/Game/Blueprints/Main/BP_PlayerState` (`Pawn.PlayerState` _asthird_person_character)))
      (set `/Game/Blueprints/Main/BP_PlayerState.Reloading` false _asbp_player_state))))

(fn `UserConstructionScript`)