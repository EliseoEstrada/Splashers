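; BP_PowerUp is a single-use pickup that grants a temporary big-projectile power-up to the player who touches it.
; Overlapping its box with a ThirdPersonCharacter sets the BigProyectil flag on that player's BP_PlayerState and hides the mesh.
; A timeline played in reverse acts as the countdown, sending its value to the player controller through ClientUpdatePowerUp.
; When it finishes, the flag is cleared and the actor destroys itself.
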(event `self.Box.OnComponentBeginOverlap`
  (params (OverlappedComponent :type "PrimitiveComponent Object Reference") (OtherActor :type "Actor Object Reference") (OtherComp :type "PrimitiveComponent Object Reference") (OtherBodyIndex :type Integer) (bFromSweep :type Boolean) (SweepResult :type "HitResult Structure (by ref)"))
  (if (not (`self.active`))
    (cast `/Game/ThirdPersonBP/Blueprints/ThirdPersonCharacter` OtherActor)
    (bind _asbp_player_controller (cast `/Game/Blueprints/Main/BP_PlayerController` (`self.GetInstigatorController` OtherActor)))
    (set `self.active` true)
    (bind _playerstate (`Controller.PlayerState` _asbp_player_controller))
    (bind _asbp_player_state (cast `/Game/Blueprints/Main/BP_PlayerState` _playerstate))
    (set `/Game/Blueprints/Main/BP_PlayerState.Big Proyectil` true _asbp_player_state)
    (`SceneComponent.SetHiddenInGame` (`self.StaticMesh`) true false)
    (bind (_direction _newtrack_0) (`Timeline|Timeline_0` :!via `ReverseFromEnd`)
      (:`Update`
        (`/Game/Blueprints/Main/BP_PlayerController.Client Update Power Up` _asbp_player_controller _newtrack_0))
      (:`Finished`
        (bind _asbp_player_state_2 (cast `/Game/Blueprints/Main/BP_PlayerState` _playerstate))
        (set `/Game/Blueprints/Main/BP_PlayerState.Big Proyectil` false _asbp_player_state_2)
        (`self.K2_DestroyActor`)))))

(fn `UserConstructionScript`)